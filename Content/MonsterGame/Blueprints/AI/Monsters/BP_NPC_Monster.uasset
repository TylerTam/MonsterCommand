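; Monster NPC that picks targets, computes movement along navmesh paths and hides itself when it dies.
; AI Perception maintains a list of spotted actors; each tick it caches a current target, preferring an assigned override over the closest spotted one.
; Paths are built synchronously on request, and GetDesiredVelocity steps through their points within a stopping distance, returning a unit direction.
; A control-input movement branch remains but is disabled by a constant condition.
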(event `self.ReceiveTick`
  (params (DeltaSeconds :type "Float (single-precision)"))
  (set `self.(Temp) Target` (`self.GetCurrentTarget`)))

(event `CreateNewPath`
  (params (TargetLocation :type "Vector Structure"))
  (bind _returnvalue (`NavigationSystemV1.FindPathToLocationSynchronously` (`self.K2_GetActorLocation`) TargetLocation null null))
  (set `self.NavPath` _returnvalue)
  (set `self.NavPathIndex` 1)
  (set `self.ReachedPath` false))

(event `self.Health.OnIDied`
  (`self.SetActorHiddenInGame` self true))

(event `self.AIPerception.OnPerceptionUpdated`
  (params (UpdatedActors :type "Array of Actor Object Reference (by ref)"))
  (bind _spottedtargets (`self.SpottedTargets`))
  (for _array_element UpdatedActors
    (bind _info (`AIPerceptionComponent.GetActorsPerception` (`self.AIPerception`) _array_element))
    (if (`.bSuccessfullySensed` (break `AIStimulus` (`|GetArrayItem` (`.LastSensedStimuli` (break `ActorPerceptionBlueprintInfo` _info)))))
      (bind _returnvalue (`KismetArrayLibrary.Array_Contains` _spottedtargets _array_element))
      (if (not _returnvalue)
        (`KismetArrayLibrary.Array_Add` _spottedtargets _array_element))
      (elif _returnvalue
        (`KismetArrayLibrary.Array_RemoveItem` _spottedtargets _array_element)))))

(event `self.SelectableEntity_AI.OnOverrideTargetAssigned`
  (params (newTarget :type "Actor Object Reference"))
  (set `self.OverrideTarget` newTarget))

(fn `GetClosestTarget`
  (returns (ClosestTarget :type "Actor Object Reference"))
  (locals (Closest :type "Actor Object Reference"))
  (bind _returnvalue (`self.K2_GetActorLocation` self))
  (if (== (`KismetArrayLibrary.Array_Length` (`self.SpottedTargets`)) 0)
    (return null)
    (else
      (for _array_element (`self.SpottedTargets`)
        (if (== (`local.Closest`) null)
          (set `local.Closest` _array_element)
          (elif (< (`KismetMathLibrary.Vector_Distance` _returnvalue (`self.K2_GetActorLocation` _array_element)) (`KismetMathLibrary.Vector_Distance` (`self.K2_GetActorLocation` (`local.Closest`)) _returnvalue))
            (set `local.Closest` _array_element))))
      (return (`local.Closest`)))))

(fn `GetCurrentTarget`
  (returns (Target :type "Actor Object Reference"))
  (bind _overridetarget (`self.OverrideTarget`))
  (if (!= _overridetarget null)
    (return _overridetarget)
    (else
      (return (`self.GetClosestTarget`)))))

(fn `GetDesiredVelocity`
  (returns (TargetVelocity :type "Vector Structure"))
  (bind (_returnvalue_roll _returnvalue_pitch _returnvalue_yaw) (`KismetMathLibrary.BreakRotator` (`self.GetControlRotation`)))
  (bind _returnvalue (`self.K2_GetActorLocation`))
  (bind _navpathindex (`self.NavPathIndex`))
  (bind _pathpoints (`NavigationPath.PathPoints` (`self.NavPath`)))
  (bind _output (`|GetArrayItem` _pathpoints _navpathindex))
  (if true
    (if (not (`self.ReachedPath`))
      (if (< _navpathindex (`KismetArrayLibrary.Array_Length` _pathpoints))
        (if (<= (`KismetMathLibrary.Vector_Distance` _returnvalue _output) (`self.StoppingDistance`))
          (`/Engine/EditorBlueprintResources/StandardMacros.IncrementInt` (`self.NavPathIndex`))
          (else
            (return (`KismetMathLibrary.GetDirectionUnitVector` _returnvalue _output))))
        (else
          (set `self.ReachedPath` true)
          (return (0.0 0.0 0.0))))
      (else
        (return (0.0 0.0 0.0))))
    (else
      (return (+ (* (`KismetMathLibrary.GetForwardVector` (`KismetMathLibrary.MakeRotator` 0.0 0.0 _returnvalue_yaw)) (`self.GetInputAxisValue`)) (* (`KismetMathLibrary.GetRightVector` (`KismetMathLibrary.MakeRotator` 0.0 0.0 _returnvalue_yaw)) (`self.GetInputAxisValue`)))))))

(fn `GetTargetLoation`
  (returns (TargetPosition :type "Vector Structure") (ReachedPos :type Boolean))
  (bind _navpath (`self.NavPath`))
  (bind _navpathindex (`self.NavPathIndex`))
  (bind _pathpoints (`NavigationPath.PathPoints` _navpath))
  (if (!= _navpath null)
    (if (`NavigationPath.IsValid` _navpath)
      (if (< _navpathindex (`KismetArrayLibrary.Array_Length` _pathpoints))
        (return (`|GetArrayItem` _pathpoints _navpathindex) false)
        (else
          _))))
  (return (`self.K2_GetActorLocation`) true))

(fn `ReachedEndOfNavMesh`
  (returns (NewParam :type Boolean))
  (bind _navpath (`self.NavPath`))
  (if (!= _navpath null)
    (if (`NavigationPath.IsValid` _navpath)
      (if (< (`self.NavPathIndex`) (`KismetArrayLibrary.Array_Length` (`NavigationPath.PathPoints` _navpath)))
        _
        (else
          (return true))))
    (return false)
    (else
      (return true))))

(fn `SetLocationTarget`
  (params (TargetPos :type "Vector Structure"))
  (returns (ReachedDestination :type Boolean))
  (bind _returnvalue (`self.K2_GetActorLocation`))
  (`NavigationSystemV1.FindPathToLocationSynchronously` (`NavigationSystemV1.GetNavigationSystem`) _returnvalue TargetPos null null)
  (return (<= (`KismetMathLibrary.Vector_Distance` TargetPos _returnvalue) (`self.StoppingDistance`))))

(fn `UserConstructionScript`)