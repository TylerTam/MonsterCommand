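; BP_Player is the player Blueprint that turns input actions into commands for controlling monsters.
; It forwards Select press and release, four indexed attack slots, Summon and Return to a CommandManager.
; The Blueprint holds no gameplay logic of its own, leaving the handling of each command to that manager.
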(event `InputAction|Select`
  (params (Key :type "Key Structure"))
  (bind _commandmanager (`self.CommandManager`))
  (:`Pressed`
    (`CommandManager.SelectPressed` _commandmanager))
  (:`Released`
    (`CommandManager.SelectReleased` _commandmanager)))

(event `InputAction|Attack1`
  (params (Key :type "Key Structure"))
  (:`Pressed`
    (`CommandManager.AttackPressed` (`self.CommandManager`) 0)))

(event `InputAction|Attack2`
  (params (Key :type "Key Structure"))
  (:`Pressed`
    (`CommandManager.AttackPressed` (`self.CommandManager`) 1)))

(event `InputAction|Attack3`
  (params (Key :type "Key Structure"))
  (:`Pressed`
    (`CommandManager.AttackPressed` (`self.CommandManager`) 2)))

(event `InputAction|Attack4`
  (params (Key :type "Key Structure"))
  (:`Pressed`
    (`CommandManager.AttackPressed` (`self.CommandManager`) 3)))

(event `InputAction|Summon`
  (params (Key :type "Key Structure"))
  (:`Pressed`
    (`CommandManager.SummonPressed` (`self.CommandManager`))))

(event `InputAction|Return`
  (params (Key :type "Key Structure"))
  (:`Pressed`
    (`CommandManager.ReturnMonsterPressed` (`self.CommandManager`))))

(fn `UserConstructionScript`)